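; Gameplay game mode for a Rebel versus Militia match, spawning each player as a demonstrator or cop pawn by team.
; A looping timer drives a five-minute countdown, which Tick formats for player state 0's timer.
; Tick also counts Poster actors every frame: none left means Rebels win, time running out means Militia wins.
; Either ending notifies the game state, then server-travels to the lobby after a short delay.
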(event `self.ReceiveBeginPlay`
  (set `self.RemainingTime` 300)
  (bind _returnvalue (`KismetSystemLibrary.K2_SetTimer` null "UpdateTimer" 1.0 true))
  (set `self.TimerHandle` _returnvalue))

(event `GameEnd_Rebel`
  (`/Engine/EditorBlueprintResources/StandardMacros.DoOnce` false
    (:`Completed`
      (bind _asbp_gs_base (cast `/Game/Gameplay/BP_GS_Base` (`GameplayStatics.GetGameState`)))
      (`/Game/Gameplay/BP_GS_Base.EndGame_Rebel` _asbp_gs_base)
      (`KismetSystemLibrary.Delay` 5.0 :!label _label)
      (set `self.RemainingTime` 300)
      (set `self.RemainingPosters` 1)
      (`AdvancedSessionsLibrary.ServerTravel` "L_Lobby?listen"))))

(event `GameEnd_Militia`
  (`/Engine/EditorBlueprintResources/StandardMacros.DoOnce` false
    (:`Completed`
      (bind _asbp_gs_base (cast `/Game/Gameplay/BP_GS_Base` (`GameplayStatics.GetGameState`)))
      (`/Game/Gameplay/BP_GS_Base.EndGame_Militia` _asbp_gs_base)
      (goto _label))))

(event `self.ReceiveTick`
  (params (DeltaSeconds :type "Float (single-precision)"))
  (`self.TranslateTimer`)
  (if (== (`self.RemainingTime`) 0)
    (`self.GameEnd_Militia`)
    (elif (== (`self.RemainingPosters`) 0)
      (`self.GameEnd_Rebel`)
      (else
        (bind _outactors (`GameplayStatics.GetAllActorsOfClass` "/Game/Gameplay/Posters/Poster.Poster_C"))
        (bind _output_get (set `self.Posters` _outactors))
        (set `self.RemainingPosters` (`KismetArrayLibrary.Array_Length` _output_get))))))

(event `self.HandleStartingNewPlayer`
  (params (NewPlayer :type "PlayerController Object Reference"))
  (bind _asbp_player_controller (cast `/Game/Gameplay/BP_PlayerController` NewPlayer))
  (`/Game/Gameplay/BP_PlayerController.LoadTeamID` _asbp_player_controller)
  (`self.SpawnPlayers` _asbp_player_controller))

(event `TranslateTimer`
  (bind _remainingtime (`self.RemainingTime`))
  ;[0 0 0] Timer
  (bind _output_get (set `self.Minutes` (/ _remainingtime 60)))
  (bind _output_get_2 (set `self.Seconds` (mod _remainingtime 60)))
  (bind _output_get_3 (set `self.TimerUI` (`KismetStringLibrary.JoinStringArray` (`|MakeArray` (`KismetStringLibrary.Conv_IntToString` _output_get) (`KismetStringLibrary.Conv_IntToString` _output_get_2)) ":")))
  (bind _asbp_player_state (cast `/Game/Gameplay/BP_PlayerState` (`GameplayStatics.GetPlayerState` 0)))
  (`/Game/Gameplay/BP_PlayerState.UpdateTimer` _asbp_player_state _output_get_3))

(fn `ChoosePlayerStart`
  (params (Player :type "Controller Object Reference"))
  (returns (ReturnValue :type "Actor Object Reference"))
  (bind _asbp_player_controller (cast `/Game/Gameplay/BP_PlayerController` Player))
  (bind _outactors (`GameplayStatics.GetAllActorsOfClass` "/Script/Engine.PlayerStart"))
  (for _array_element _outactors
    (if (== (`PlayerStart.PlayerStartTag` _array_element) (`/Game/Gameplay/BP_PlayerController.TeamID` _asbp_player_controller))
      (return _array_element))))

(fn `SpawnPlayers`
  (params (Player :type "/Game/Gameplay/BP_PlayerController Object Reference"))
  (bind _returnvalue (`self.GetTransform` Player))
  (`KismetArrayLibrary.Array_Add` (`self.All_PlayerControllers`) Player)
  (switch `name` (`/Game/Gameplay/BP_PlayerController.TeamID` Player)
    (:`Rebel`
      (bind _returnvalue_2 (`|SpawnActorFromClass` "/Game/Gameplay/GameplayCharacters/BP_ThirdPerson_Demonstrant.BP_ThirdPerson_Demonstrant_C" _returnvalue "Undefined" "MultiplyWithRoot" null null))
      (`Controller.Possess` Player _returnvalue_2)
      (`WidgetBlueprintLibrary.SetInputMode_GameOnly` Player true)
      (set `PlayerController.bShowMouseCursor` false Player))
    (:`Militia`
      (bind _returnvalue_3 (`|SpawnActorFromClass` "/Game/Gameplay/GameplayCharacters/BP_ThirdPerson_Cop.BP_ThirdPerson_Cop_C" _returnvalue "Undefined" "MultiplyWithRoot" null null))
      (`Controller.Possess` Player _returnvalue_3)
      (`WidgetBlueprintLibrary.SetInputMode_GameOnly` Player true)
      (set `PlayerController.bShowMouseCursor` false Player))))

(fn `UpdateTimer`
  (if (> (`self.RemainingTime`) 0)
    (`/Engine/EditorBlueprintResources/StandardMacros.DecrementInt` (`self.RemainingTime`))
    (else
      (`KismetSystemLibrary.K2_ClearAndInvalidateTimerHandle` (`self.TimerHandle`)))))

(fn `UserConstructionScript`)