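; Player controller that creates the gameplay HUD widget and manages the player's team ID.
; On BeginPlay it creates WBP_Gameplay and adds it to the viewport.
; RequestTeamChange writes the new team to BP_PlayerState and caches it on the controller.
; LoadTeamID copies that cached value back into the player state.
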(event `self.ReceiveBeginPlay`
  (bind _returnvalue (`|CreateWidget` "/Game/Levels/Gameplay/WBP_Gameplay.WBP_Gameplay_C" self))
  (`UserWidget.AddToViewport` _returnvalue 0))

(event `self.ReceiveTick`
  (params (DeltaSeconds :type "Float (single-precision)")))

(event `RequestTeamChange`
  (params (NewTeamID :type Name))
  (bind _asbp_player_state (cast `/Game/Gameplay/BP_PlayerState` (`self.PlayerState`)))
  (bind _output_get (set `/Game/Gameplay/BP_PlayerState.TeamID` NewTeamID _asbp_player_state))
  (set `self.TeamID` _output_get))

(event `LoadTeamID`
  (bind _asbp_player_state (cast `/Game/Gameplay/BP_PlayerState` (`self.PlayerState`)))
  (set `/Game/Gameplay/BP_PlayerState.TeamID` (`self.TeamID`) _asbp_player_state))

(fn `UserConstructionScript`)