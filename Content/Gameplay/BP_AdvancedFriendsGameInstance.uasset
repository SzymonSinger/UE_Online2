(event `OpenLevel`
  (`GameplayStatics.OpenLevelBySoftObjectPtr` "/Game/ThirdPerson/Maps/ThirdPersonMap.ThirdPersonMap" true "listen"))

(event `CreateAdvancedSession`
  (params (SessionName :type Text))
  (bind _returnvalue (`GameplayStatics.GetPlayerController` 0))
  ;[1 1 1] Creating session
  (`DestroySessionCallbackProxy.DestroySession` _returnvalue
    (:`then`
      (`CreateSessionCallbackProxyAdvanced.CreateAdvancedSession` :`PlayerController` _returnvalue :`PublicConnections` 6
        (:`OnSuccess`
          (`KismetSystemLibrary.PrintString` "Session Created!")
          (`GameplayStatics.OpenLevelBySoftObjectPtr` "/Game/Levels/Lobby/L_Lobby.L_Lobby" true "listen"))
        (:`OnFailure`
          (`KismetSystemLibrary.PrintString` "Failed to create session!"))))
    (:`OnSuccess`
      (`KismetSystemLibrary.PrintString` "Destroyed session"))
    (:`OnFailure`
      (`KismetSystemLibrary.PrintString` "Failed to destroy session"))))

(event `JoinAdvancedSession`
  (bind _returnvalue (`GameplayStatics.GetPlayerController` 0))
  (bind _results (`FindSessionsCallbackProxy.FindSessions` _returnvalue 1)
    (:`then`
      (`KismetSystemLibrary.PrintString` "Looking for Sessions!"))
    (:`OnSuccess`
      (bind _output_get (set `self.Results` _results))
      (`JoinSessionCallbackProxy.JoinSession` _returnvalue (`|GetArrayItem` _output_get)
        (:`OnSuccess`
          (`KismetSystemLibrary.PrintString` "Session found! Joining"))
        (:`OnFailure`
          (`KismetSystemLibrary.PrintString` "Session not found!"))))))

(event `DestroyAdvancedSession`
  (`DestroySessionCallbackProxy.DestroySession` (`GameplayStatics.GetPlayerController` 0)
    (:`OnSuccess`
      (`KismetSystemLibrary.PrintString` "Destroyed session"))
    (:`OnFailure`
      (`KismetSystemLibrary.PrintString` "Failed to destroy session"))))

(event `self.OnSessionInviteAccepted`
  (params (LocalPlayerNum :type Integer) (PersonInvited :type "BPUniqueNetId Structure") (SessionToJoin :type "BlueprintSessionResult Structure (by ref)"))
  (bind _returnvalue (`GameplayStatics.GetPlayerController` 0))
  ;[1 1 1] Invitation Handling
  (`DestroySessionCallbackProxy.DestroySession` _returnvalue
    (:`then`
      (`KismetSystemLibrary.PrintString` "Invite Accepted, joining session")
      (`JoinSessionCallbackProxy.JoinSession` _returnvalue SessionToJoin
        (:`OnSuccess`
          (`KismetSystemLibrary.PrintString` "Joining session!"))
        (:`OnFailure`
          (`KismetSystemLibrary.PrintString` "Failed to join session"))))))

(event `self.OnSessionInviteReceived`
  (params (LocalPlayerNum :type Integer) (PersonInviting :type "BPUniqueNetId Structure") (AppId :type String) (SessionToJoin :type "BlueprintSessionResult Structure (by ref)"))
  (bind _returnvalue (`GameplayStatics.GetPlayerController` 0))
  ;[1 1 1] Invitation Handling
  (`DestroySessionCallbackProxy.DestroySession` _returnvalue
    (:`then`
      (`KismetSystemLibrary.PrintString` "Invite Received, joining session")
      (`JoinSessionCallbackProxy.JoinSession` _returnvalue SessionToJoin
        (:`OnSuccess`
          (`KismetSystemLibrary.PrintString` "Joining session!"))
        (:`OnFailure`
          (`KismetSystemLibrary.PrintString` "Failed to join session"))))))