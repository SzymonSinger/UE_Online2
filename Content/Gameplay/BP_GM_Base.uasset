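; BP_GM_Base is a base game mode that tracks connected players and supports server travel.
; It adds or removes player controllers on login and logout, then triggers a player list update.
; Update_PlayerList waits briefly before asking BP_GS_Base, the game state, to update its list.
; It also has each starting player controller load its team ID and exposes an event for absolute ServerTravel to a given URL.
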(event `Update_PlayerList`
  (`KismetSystemLibrary.Delay` 0.3)
  (bind _asbp_gs_base (cast `/Game/Gameplay/BP_GS_Base` (`GameplayStatics.GetGameState`)))
  (`/Game/Gameplay/BP_GS_Base.Update_PlayerList` _asbp_gs_base))

(event `self.K2_PostLogin`
  (params (NewPlayer :type "PlayerController Object Reference"))
  (bind _asbp_player_controller (cast `/Game/Gameplay/BP_PlayerController` NewPlayer))
  (`KismetArrayLibrary.Array_Add` (`self.All_PlayerControllers`) _asbp_player_controller)
  (`self.Update_PlayerList` :!label _label))

(event `self.K2_OnLogout`
  (params (ExitingController :type "Controller Object Reference"))
  (bind _asbp_player_controller (cast `/Game/Gameplay/BP_PlayerController` ExitingController))
  (`KismetArrayLibrary.Array_RemoveItem` (`self.All_PlayerControllers`) _asbp_player_controller)
  (goto _label))

(event `self.HandleStartingNewPlayer`
  (params (NewPlayer :type "PlayerController Object Reference"))
  (bind _asbp_player_controller (cast `/Game/Gameplay/BP_PlayerController` NewPlayer))
  (`/Game/Gameplay/BP_PlayerController.LoadTeamID` _asbp_player_controller))

(event `ServerTravel`
  (params (`In URL` :type String))
  (`AdvancedSessionsLibrary.ServerTravel` `In URL` true))

(fn `UserConstructionScript`)