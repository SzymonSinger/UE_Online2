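; BP_GS_Base is a game state Blueprint that maintains the player list for the lobby and broadcasts Rebel or Militia end-of-game events.
; Update_PlayerList copies PlayerArray into AllPlayerStates and sets each BP_PlayerState's name from its controller.
; The list's RepNotify refreshes every WBP_Lobby widget.
; The two EndGame events loop over PlayerArray and call the matching EndReb or EndMil on each BP_PlayerController.
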(event `Update_PlayerList`
  (bind _output_get (set `self.All_PlayerStates` (`self.PlayerArray`)))
  (for _array_element _output_get
    (bind _asbp_player_state (cast `/Game/Gameplay/BP_PlayerState` _array_element))
    (set `/Game/Gameplay/BP_PlayerState.PlayerName` (`AdvancedSessionsLibrary.GetPlayerName` (`PlayerState.GetPlayerController` _array_element)) _asbp_player_state)))

(event `EndGame_Rebel`
  (for _array_element (`self.PlayerArray`)
    (bind _asbp_player_controller (cast `/Game/Gameplay/BP_PlayerController` (`PlayerState.GetPlayerController` _array_element)))
    (`/Game/Gameplay/BP_PlayerController.EndReb` _asbp_player_controller)))

(event `EndGame_Militia`
  (for _array_element (`self.PlayerArray`)
    (bind _asbp_player_controller (cast `/Game/Gameplay/BP_PlayerController` (`PlayerState.GetPlayerController` _array_element)))
    (`/Game/Gameplay/BP_PlayerController.EndMil` _asbp_player_controller)))

(fn `OnRep_All_PlayerStates`
  (bind _foundwidgets (`WidgetBlueprintLibrary.GetAllWidgetsOfClass` "/Game/Levels/Lobby/WBP_Lobby.WBP_Lobby_C" false))
  (for _array_element _foundwidgets
    (`/Game/Levels/Lobby/WBP_Lobby.Update_Widget` _array_element)))

(fn `UserConstructionScript`)