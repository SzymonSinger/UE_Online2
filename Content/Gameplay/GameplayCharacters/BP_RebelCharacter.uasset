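; Rebel character Blueprint that starts ripping posters when the camera points at one within short range.
; Each Tick, it line traces from the mesh's head socket along the follow camera's forward vector, with debug drawing on.
; A hit actor tagged as a poster is cast to Poster and told to StartRipping, with no input check or repeat guard here.
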(event `InputAction|Interact`
  (params (Key :type "Key Structure")))

(event `self.ReceiveTick`
  (params (DeltaSeconds :type "Float (single-precision)"))
  (bind _returnvalue (`SceneComponent.GetSocketLocation` (`self.Mesh`) "headSocket"))
  (bind (_outhit _returnvalue_2) (`KismetSystemLibrary.LineTraceSingle` :`Start` _returnvalue :`End` (+ _returnvalue (* (`KismetMathLibrary.GetForwardVector` (`SceneComponent.K2_GetComponentRotation` (`self.FollowCamera`))) 200.0)) :`TraceChannel` "TraceTypeQuery3" :`DrawDebugType` "ForDuration"))
  (if _returnvalue_2
    (bind (_bblockinghit _binitialoverlap _time _distance _location _impactpoint _normal _impactnormal _physmat _hitactor) (`GameplayStatics.BreakHitResult` _outhit))
    (if (`self.ActorHasTag` _hitactor "Poster")
      (bind _asposter (cast `/Game/Gameplay/Posters/Poster` _hitactor))
      (`/Game/Gameplay/Posters/Poster.StartRipping` _asposter))))

(fn `UserConstructionScript`)